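; Player pawn Blueprint that handles movement input and stubs out fire, secondary fire and pause actions with debug prints.
; BeginPlay enables input and adds the Enhanced Input mapping context to the first player controller's subsystem.
; IA_Up and IA_Right add movement relative to control yaw, reading the action value's X and Y respectively.
; Legacy Up and Right axis events remain alongside them, moving along fixed zero-yaw world directions.
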(event `self.ReceiveBeginPlay`
  (bind _returnvalue (`GameplayStatics.GetPlayerController` 0))
  (`self.EnableInput` _returnvalue)
  (bind _asplayer_controller (cast `PlayerController` _returnvalue))
  (bind _returnvalue_2 (pcsubsystem `EnhancedInputLocalPlayerSubsystem` _asplayer_controller))
  (`/Engine/EditorBlueprintResources/StandardMacros.IsValid` _returnvalue_2
    (:`Is Valid`
      (`EnhancedInputSubsystemInterface.AddMappingContext` _returnvalue_2 "/Game/Migrate/Inputs/InputMapping.InputMapping" 0 (struct)))))

(event `EnhancedInput|/Game/Migrate/Inputs/IA_Fire`
  (params (ActionValue :type Boolean) (ElapsedSeconds :type "Float (double-precision)") (TriggeredSeconds :type "Float (double-precision)") (InputAction :type "InputAction Object Reference" :default "/Game/Migrate/Inputs/IA_Fire.IA_Fire"))
  (:`Triggered`
    (`KismetSystemLibrary.PrintString` "Shoot !!")))

(event `EnhancedInput|/Game/Migrate/Inputs/IA_SecondaryFire`
  (params (ActionValue :type Boolean) (ElapsedSeconds :type "Float (double-precision)") (TriggeredSeconds :type "Float (double-precision)") (InputAction :type "InputAction Object Reference" :default "/Game/Migrate/Inputs/IA_SecondaryFire.IA_SecondaryFire"))
  (:`Started`
    (`KismetSystemLibrary.PrintString` "Secondary Fire !!!")))

(event `InputAxis|Up`
  (params (AxisValue :type "Float (single-precision)"))
  (`self.AddMovementInput` (`KismetMathLibrary.GetForwardVector` (`KismetMathLibrary.MakeRotator` 0.0 0.0 (.yaw (struct)))) AxisValue))

(event `EnhancedInput|/Game/Migrate/Inputs/IA_Pause`
  (params (ActionValue :type Boolean) (ElapsedSeconds :type "Float (double-precision)") (TriggeredSeconds :type "Float (double-precision)") (InputAction :type "InputAction Object Reference" :default "/Game/Migrate/Inputs/IA_Pause.IA_Pause"))
  (:`Started`
    (`KismetSystemLibrary.PrintString` "Pause")))

(event `InputAxis|Right`
  (params (AxisValue :type "Float (single-precision)"))
  (`self.AddMovementInput` (`KismetMathLibrary.GetRightVector` (`KismetMathLibrary.MakeRotator` 0.0 0.0 (.yaw (struct)))) AxisValue))

(event `EnhancedInput|/Game/Migrate/Inputs/IA_Up`
  (params (ActionValue :type "Vector2D Structure") (ElapsedSeconds :type "Float (double-precision)") (TriggeredSeconds :type "Float (double-precision)") (InputAction :type "InputAction Object Reference" :default "/Game/Migrate/Inputs/IA_Up.IA_Up"))
  (:`Triggered`
    (`self.AddMovementInput` (`KismetMathLibrary.GetForwardVector` (`KismetMathLibrary.MakeRotator` 0.0 0.0 (.yaw (`self.GetControlRotation`)))) ActionValue_X)))

(event `EnhancedInput|/Game/Migrate/Inputs/IA_Right`
  (params (ActionValue :type "Vector2D Structure") (ElapsedSeconds :type "Float (double-precision)") (TriggeredSeconds :type "Float (double-precision)") (InputAction :type "InputAction Object Reference" :default "/Game/Migrate/Inputs/IA_Right.IA_Right"))
  (:`Triggered`
    (`self.AddMovementInput` (`KismetMathLibrary.GetRightVector` (`KismetMathLibrary.MakeRotator` 0.0 0.0 (.yaw (`self.GetControlRotation`)))) ActionValue_Y)))

(fn `UserConstructionScript`)