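; Player ship actor that shares hit, collector and particle state with a mobile companion through sync objects.
; On game start it creates the life bar UI; enemy overlaps and mobile-reported hits deal damage, though Kill is empty.
; Weapon part overlaps fill the collector if empty.
; Tick polls synced state for hits and room scans, which randomize particle color, shape and rotation via a dynamic material and publish indices as the right-computer answer.
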(event `RandoParticles_Event`
  (bind _returnvalue (`KismetMaterialLibrary.CreateDynamicMaterialInstance` (`self.ParticleBaseMaterial`)))
  (set `self.DynamicParticleMaterial` _returnvalue)
  (`self.RandomizeParticles`))

(event `self.ReceiveBeginPlay`
  (bind _returnvalue (`KismetMaterialLibrary.CreateDynamicMaterialInstance` (`self.ParticleBaseMaterial`)))
  (set `self.DynamicParticleMaterial` _returnvalue)
  (set `self.CurrentHealth` (`self.StartHealth`))
  (bind _outactors (`GameplayStatics.GetAllActorsOfClass` "/Game/Blueprints/Network/GameManager.GameManager_C"))
  (for (_array_element _array_index) _outactors
    (if (== _array_index 0)
      (add `/Game/Blueprints/Network/GameManager.OnGameStart` _array_element (delegate `OnGameStart_Event`)))))

(event `self.ReceiveTick`
  (params (DeltaSeconds :type "Float (single-precision)"))
  (`self.UpdateShipParticles`)
  (`self.UpdateWasHitFromMobile`))

(event `self.Collider.OnComponentBeginOverlap`
  (params (OverlappedComponent :type "PrimitiveComponent Object Reference") (OtherActor :type "Actor Object Reference") (OtherComp :type "PrimitiveComponent Object Reference") (OtherBodyIndex :type Integer) (bFromSweep :type Boolean) (SweepResult :type "HitResult Structure (by ref)"))
  (`self.CheckCollisionWithWeaponPart` OtherActor)
  (`self.CheckCollisionWithEnemy` OtherActor))

(event `OnGameStart_Event`
  (bind _returnvalue (`|CreateWidget` "/Game/UI/MainUI.MainUI_C"))
  (bind _output_get (set `self.MainUI` _returnvalue))
  (`UserWidget.AddToViewport` _output_get 0)
  (`/Game/UI/MainUI.UpdateLifeBar` _output_get (`self.CurrentHealth`)))

(fn `CheckCollisionWithEnemy`
  (params (CollidedActor :type "Actor Object Reference"))
  (bind _asenemy_actor (cast `EnemyActor` CollidedActor))
  (`self.TakeDamage` (`EnemyActor.ContactDamage` _asenemy_actor)))

(fn `CheckCollisionWithWeaponPart`
  (params (CollidedActor :type "Actor Object Reference"))
  (bind _iscollectorfull (`CollectorSyncComponent.IsCollectorFull` (`self.CollectorSync`)))
  (bind _asweapon_part (cast `/Game/Blueprints/WeaponPart` CollidedActor))
  (if (not (`SynchronizedBool.GetValue` _iscollectorfull))
    (bind _output_get (set `self.True` true))
    (`SynchronizedBool.SetValue` _iscollectorfull _output_get)
    (`self.K2_DestroyActor` _asweapon_part)))

(fn `Kill`)

(fn `RandomizeParticles`
  (bind _dynamicparticlematerial (`self.DynamicParticleMaterial`))
  (bind (_outitem _outindex) (`KismetArrayLibrary.Array_Random` (`self.ParticleShapes`)))
  (bind (_outitem_2 _outindex_2) (`KismetArrayLibrary.Array_Random` (`self.ParticleColors`)))
  (bind (_outitem_3 _outindex_3) (`KismetArrayLibrary.Array_Random` (`self.ParticleRotation`)))
  (bind (_returnvalue_roll _returnvalue_pitch _returnvalue_yaw) (`KismetMathLibrary.BreakRotator` (`SceneComponent.K2_GetComponentRotation` (`self.DefaultSceneRoot`))))
  (`MaterialInstanceDynamic.SetVectorParameterValue` _dynamicparticlematerial "ParticlesColor" (`KismetMathLibrary.Conv_ColorToLinearColor` _outitem_2))
  (`MaterialInstanceDynamic.SetTextureParameterValue` _dynamicparticlematerial "ParticlesShape" _outitem)
  (`SceneComponent.K2_SetWorldRotation` (`self.ShipParticle`) (`KismetMathLibrary.MakeRotator` (+ _returnvalue_roll _outitem_3) (+ _returnvalue_pitch -90.0) _returnvalue_yaw) false false)
  (`NiagaraComponent.SetVariableMaterial` (`self.ShipParticle`) "ParticleMaterial" (`self.DynamicParticleMaterial`))
  (`SynchronizedFIntVector.SetValue` (`ShipParticlesSyncComponent.RightComputerResultAnswer` (`self.ShipParticlesSync`)) (make `IntVector` _outindex_2 _outindex_3 _outindex))
  (set `self.ParticleDisplayed` true)
  (`NiagaraComponent.SetPaused` (`self.ShipParticle`) false))

(fn `ResetIsPlayerHitIfNeeded`
  (bind _isplayerhit (`PlayerHitSyncComponent.IsPlayerHit` (`self.PlayerHitSync`)))
  (if (`self.WasPlayerJustHit`)
    (bind _returnvalue (`SpecializedSynchronizedProperty.NeedSync` _isplayerhit))
    (if _returnvalue
      (bind _output_get (set `self.False` false))
      (`SynchronizedBool.SetValue` _isplayerhit _output_get)
      (set `self.WasPlayerJustHit` false))))

(fn `TakeDamage`
  (params (damagesTaken :type Integer) (`From mobile` :type Boolean))
  (if (not `From mobile`)
    (bind _output_get (set `self.True` true))
    (`SynchronizedBool.SetValue` (`PlayerHitSyncComponent.IsPlayerHit` (`self.PlayerHitSync`)) _output_get)
    (set `self.WasPlayerJustHit` true))
  (bind _output_get_2 (set `self.CurrentHealth` (- (`self.CurrentHealth`) damagesTaken)))
  (if (<= _output_get_2 0)
    (`self.Kill`)
    (else
      (`/Game/UI/MainUI.UpdateLifeBar` (`self.MainUI`) _output_get_2))))

(fn `UpdateShipParticles`
  (bind _returnvalue (`SynchronizedBool.GetValue` (`ShipParticlesSyncComponent.IsRoomScanned` (`self.ShipParticlesSync`))))
  (if (!= _returnvalue (`self.ParticleDisplayed`))
    (if _returnvalue
      (`self.RandomizeParticles`))
    (`NiagaraComponent.SetPaused` (`self.ShipParticle`) (not _returnvalue))))

(fn `UpdateWasHitFromMobile`
  (bind _isplayerhit (`PlayerHitSyncComponent.IsPlayerHit` (`self.PlayerHitSync`)))
  (if (`SynchronizedBool.GetValue` _isplayerhit)
    (bind _returnvalue (`SpecializedSynchronizedProperty.NeedSync` _isplayerhit))
    (if (`KismetMathLibrary.BooleanNOR` _returnvalue (`self.WasPlayerJustHit`))
      (`SynchronizedBool.SetValue` _isplayerhit (`self.False`))
      (`self.TakeDamage` 1 true))
    (else
      (set `self.WasPlayerJustHit` false))))

(fn `UserConstructionScript`)