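; WeaponPart is an actor that drifts across the XY plane and bounces inside a rectangular area.
; BeginPlay picks a random normalized 2D direction, and Tick moves the actor along it by Speed with a swept SetActorLocation, keeping Z unchanged.
; CheckLimits then clamps X and Y to the LowerLeftLimit and UpperRightLimit bounds, flipping that axis of the direction whenever one is crossed.
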(event `self.ReceiveBeginPlay`
  (set `self.Direction` (`KismetMathLibrary.Normal2D` (`KismetMathLibrary.MakeVector2D` (`KismetMathLibrary.RandomFloatInRange` -1.0 1.0) (`KismetMathLibrary.RandomFloatInRange` -1.0 1.0)))))

(event `self.ReceiveTick`
  (params (DeltaSeconds :type "Float (single-precision)"))
  (`self.MoveAlongDirection` DeltaSeconds)
  (`self.CheckLimits`))

(fn `CheckLimits`
  (locals (X :type "Float (double-precision)") (Y :type "Float (double-precision)"))
  (bind (_returnvalue_x _returnvalue_y) (`KismetMathLibrary.BreakVector` (`self.K2_GetActorLocation`)))
  (bind (_returnvalue_x_2 _returnvalue_y_2 _returnvalue_z) (`KismetMathLibrary.BreakVector` (`self.K2_GetActorLocation`)))
  (bind (_returnvalue_x_3 _returnvalue_y_3 _returnvalue_z_2) (`KismetMathLibrary.BreakVector` (`self.K2_GetActorLocation`)))
  (bind (_direction_x _direction_y) (`KismetMathLibrary.BreakVector2D` (`self.Direction`)))
  (bind (_direction_x_2 _direction_y_2) (`KismetMathLibrary.BreakVector2D` (`self.Direction`)))
  (bind (_lowerleftlimit_x _lowerleftlimit_y) (`KismetMathLibrary.BreakVector2D` (`self.LowerLeftLimit`)))
  (bind (_lowerleftlimit_x_2 _lowerleftlimit_y_2) (`KismetMathLibrary.BreakVector2D` (`self.LowerLeftLimit`)))
  (bind (_upperrightlimit_x _upperrightlimit_y) (`KismetMathLibrary.BreakVector2D` (`self.UpperRightLimit`)))
  (bind (_upperrightlimit_x_2 _upperrightlimit_y_2) (`KismetMathLibrary.BreakVector2D` (`self.UpperRightLimit`)))
  (bind _returnvalue (< _returnvalue_y _lowerleftlimit_y_2))
  (bind _returnvalue_2 (< _returnvalue_x _lowerleftlimit_x_2))
  (if (or _returnvalue_2 (> _returnvalue_x _upperrightlimit_x))
    (set `self.Direction` (`KismetMathLibrary.MakeVector2D` (* -1.0 _direction_x_2) _direction_y_2))
    (if _returnvalue_2
      (set `local.X` _lowerleftlimit_x)
      (else
        (set `local.X` _upperrightlimit_x_2)))
    (`self.K2_SetActorLocation` (`KismetMathLibrary.MakeVector` (`local.X`) _returnvalue_y_2 _returnvalue_z)))
  (if (or _returnvalue (> _returnvalue_y _upperrightlimit_y))
    (set `self.Direction` (`KismetMathLibrary.MakeVector2D` _direction_x (* _direction_y -1.0)))
    (if _returnvalue
      (set `local.Y` _lowerleftlimit_y)
      (else
        (set `local.Y` _upperrightlimit_y_2)))
    (`self.K2_SetActorLocation` (`KismetMathLibrary.MakeVector` _returnvalue_x_3 (`local.Y`) _returnvalue_z_2))))

(fn `MoveAlongDirection`
  (params (DeltaTime :type "Float (double-precision)"))
  (bind (_returnvalue_x _returnvalue_y _returnvalue_z) (`KismetMathLibrary.BreakVector` (`self.K2_GetActorLocation`)))
  (bind _returnvalue (* DeltaTime (`self.Speed`)))
  (bind (_returnvalue_x_2 _returnvalue_y_2) (`KismetMathLibrary.BreakVector2D` (+ (`KismetMathLibrary.MakeVector2D` _returnvalue_x _returnvalue_y) (* (`KismetMathLibrary.MakeVector2D` _returnvalue _returnvalue) (`self.Direction`)))))
  (`self.K2_SetActorLocation` (`KismetMathLibrary.MakeVector` _returnvalue_x_2 _returnvalue_y_2 _returnvalue_z) true))

(fn `UserConstructionScript`)