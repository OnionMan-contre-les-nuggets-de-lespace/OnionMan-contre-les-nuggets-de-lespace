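; Game manager Blueprint for OnionMan that runs the host-side session from main menu through level sequence to game end.
; The menu opens a UDP receive socket; the first valid message is acknowledged, opening a send socket back to the client.
; While connected, Tick sends NetworkManager's encoded batches and received bytes feed back into it.
; Starting the game toggles actor visibility, chains levels via finish events, swaps music and updates synced GameState.
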(event `self.ReceiveBeginPlay`
  ;[1 1 1] Start
  (`self.SetActorsHidden` (`self.ActorsToEnableOnceConnected`) true)
  (`self.SetActorsHidden` (`self.ActorsToDisableOnceConnected`))
  (set `self.Game State` (`GameStateSyncComponent.GameState` (`self.GameStateSync`)))
  (bind _returnvalue (`|CreateWidget` "/Game/UI/MainMenu.MainMenu_C"))
  (bind _output_get (set `self.MainMenu` _returnvalue))
  (`UserWidget.AddToViewport` _output_get 0)
  (add `/Game/UI/MainMenu.OnStartServerButtonClicked` _output_get (delegate `OpenServer`))
  (`SynchronizedInt.SetValue` (`self.Game State`) (`self.WatingForGameToStartValue`))
  (`self.SetActorHiddenInGame` (`self.OnionMan`) true)
  (bind _returnvalue_2 (`GameplayStatics.SpawnSound2D` "/Game/TwinStick/Audio/Menu/OnionMan_Menu_full__Cue.OnionMan_Menu_full__Cue" 1.0 1.0 0.0 null))
  (bind _output_get_2 (set `self.MenuSound` _returnvalue_2))
  (`ActorComponent.SetActive` _output_get_2 true false))

(event `OpenServer`
  (bind _udpcomponent (`self.UDPComponent`))
  (bind (_sendip _sendport _sendboundport _sendboundip _receiveip _receiveport) (break `UDPSettings` (`UDPComponent.Settings` _udpcomponent)))
  ;[1 1 1] OpenServer
  (remove `/Game/UI/MainMenu.OnStartServerButtonClicked` (`self.MainMenu`) (delegate `OpenServer`))
  (bind _asonion_man_game_instance (cast `OnionManGameInstance` (`GameplayStatics.GetGameInstance`)))
  (set `self.NetworkManager` (`OnionManGameInstance.NetworkManager` _asonion_man_game_instance))
  (bind _returnvalue (`UDPComponent.OpenReceiveSocket` _udpcomponent _receiveip _receiveport))
  (`KismetSystemLibrary.LogString` (`KismetTextLibrary.Conv_TextToString` (`|FormatText` "[UDP] Open Recieve Socket : {bool}" _returnvalue)))
  (`/Game/UI/MainMenu.WaitForClientConnection` (`self.MainMenu`))
  (`self.SetActorHiddenInGame` (`self.OnionMan`) false))

(event `self.ReceiveTick`
  (params (DeltaSeconds :type "Float (single-precision)"))
  ;[1 1 1] Update
  (switch `/Game/Blueprints/Network/ConnectionState` (`self.ConnectionState`)
    (:`NewEnumerator1`
      (bind (_outnetworkbatches _returnvalue) (`NetworkManager.TryEncodeObjects` (`self.NetworkManager`)))
      (if _returnvalue
        (for _array_element _outnetworkbatches
          (bind _returnvalue_2 (`UDPComponent.EmitBytes` (`self.UDPComponent`) (`NetworkBatch.EncodedBatch` _array_element)))
          (if _returnvalue_2
            (`KismetSystemLibrary.LogString` "Successfully sent a message")
            (else
              (`KismetSystemLibrary.LogString` "Failed to send a message"))))))))

(event `self.UDPComponent.OnReceivedBytes`
  (params (Bytes :type "Array of Byte (by ref)") (IPAddress :type String) (Port :type "Integer (by ref)"))
  (bind _mainmenu (`self.MainMenu`))
  ;[1 1 1] Network Events
  (`KismetSystemLibrary.PrintString` (`KismetTextLibrary.Conv_TextToString` (`|FormatText` "RecievedBytes from IP {IP} and port {Port}" IPAddress Port)))
  (switch `/Game/Blueprints/Network/ConnectionState` (`self.ConnectionState`)
    (:`NewEnumerator0`
      (bind (_outencodedack _outip _returnvalue) (`NetworkManager.TryAcknoledge` (`self.NetworkManager`) Bytes))
      (if _returnvalue
        (bind _structout (setmembers `UDPSettings` :`StructRef` (`UDPComponent.Settings` (`self.UDPComponent`)) :`SendIP` _outip))
        (bind (_sendip _sendport) (break `UDPSettings` _structout))
        (bind _returnvalue_2 (`UDPComponent.OpenSendSocket` (`self.UDPComponent`) _sendip _sendport))
        (`KismetSystemLibrary.LogString` (`KismetTextLibrary.Conv_TextToString` (`|FormatText` "[UDP] Open Send Socket at IP {IP} and Port {Port} : {value}" _sendip _sendport _returnvalue_2)))
        (bind _returnvalue_3 (`UDPComponent.EmitBytes` (`self.UDPComponent`) _outencodedack))
        (if _returnvalue_3
          (set `self.IsInitialized` true)
          (set `self.ConnectionState` "NewEnumerator1")
          (`KismetSystemLibrary.LogString` "[UDP] Initialized")
          (add `/Game/UI/MainMenu.OnStartGameButtonClicked` _mainmenu (delegate `StartGame`))
          (`/Game/UI/MainMenu.OnClientConnected_Event` _mainmenu)
          (else
            (`KismetSystemLibrary.LogString` "Failed to Emit Acknoledge")))
        (else
          (`KismetSystemLibrary.LogString` "RecievedIp was not valid"))))
    (:`NewEnumerator1`
      (`NetworkManager.OnBytesRecieved` (`self.NetworkManager`) Bytes))))

(event `StartGame`
  (bind _levelstoplay (`self.LevelsToPlay`))
  (bind _mainmenu (`self.MainMenu`))
  (bind _menusound (`self.MenuSound`))
  (remove `/Game/UI/MainMenu.OnStartGameButtonClicked` _mainmenu (delegate `StartGame`))
  (`Widget.RemoveFromParent` _mainmenu)
  (`self.SetActorsHidden` (`self.ActorsToEnableOnceConnected`))
  (`self.SetActorsHidden` (`self.ActorsToDisableOnceConnected`) true)
  (`SynchronizedInt.SetValue` (`self.Game State`) (`self.GameStartedValue`))
  (`self.OnGameStart`)
  (bind _output_get (set `self.CurrentLevelIndex` 0))
  (if (< _output_get (`KismetArrayLibrary.Array_Length` _levelstoplay))
    (bind _output (`|GetArrayItem` _levelstoplay _output_get))
    (`/Game/Blueprints/Levels/BaseLevel.StartLevel` _output)
    (add `/Game/Blueprints/Levels/BaseLevel.OnLevelFinished` _output (delegate `OnLevelFinished_Event`))
    (if (`KismetSystemLibrary.IsValid` _menusound)
      (`ActorComponent.SetActive` _menusound false false)
      (bind _returnvalue (`GameplayStatics.CreateSound2D` "/Game/TwinStick/Audio/Level1/OnionMan-Niveau1_Cue.OnionMan-Niveau1_Cue" 1.0 1.0 0.0 null))
      (bind _output_get_2 (set `self.Level1Sound` _returnvalue))
      (`ActorComponent.SetActive` _output_get_2 true false))
    (else
      (`self.OnLastLevelFinished`))))

(event `OnLevelFinished_Event`
  (bind _currentlevelindex (`self.CurrentLevelIndex`))
  (bind _levelstoplay (`self.LevelsToPlay`))
  (remove `/Game/Blueprints/Levels/BaseLevel.OnLevelFinished` (`|GetArrayItem` _levelstoplay _currentlevelindex) (delegate `OnLevelFinished_Event`))
  (bind _result (`/Engine/EditorBlueprintResources/StandardMacros.IncrementInt` _currentlevelindex)
    (:`  `
      (if (< _result (`KismetArrayLibrary.Array_Length` _levelstoplay))
        (bind _output (`|GetArrayItem` (`self.LevelsToPlay`) _result))
        (`/Game/Blueprints/Levels/BaseLevel.StartLevel` _output)
        (add `/Game/Blueprints/Levels/BaseLevel.OnLevelFinished` _output (delegate `OnLevelFinished_Event`))
        (`ActorComponent.SetActive` (`self.Level1Sound`) false false)
        (bind _returnvalue (`GameplayStatics.SpawnSound2D` "/Game/TwinStick/Audio/Boss/OnionMan-Boss1.OnionMan-Boss1" 1.0 1.0 0.0 null))
        (bind _output_get (set `self.BossSound` _returnvalue))
        (`ActorComponent.SetActive` _output_get true false)
        (else
          (`self.OnLastLevelFinished`))))))

(fn `FinishGame`
  (params (IsGameLost :type Boolean))
  (`SynchronizedInt.SetValue` (`GameStateSyncComponent.GameState` (`self.GameStateSync`)) (`KismetMathLibrary.SelectInt` (`self.GameLostValue`) (`self.GameWonValue`) IsGameLost)))

(fn `SetActorsHidden`
  (params (Actors :type "Array of Actor Object Reference") (Hidden :type Boolean))
  (for _array_element Actors
    (`self.SetActorHiddenInGame` _array_element Hidden)))

(fn `UserConstructionScript`)