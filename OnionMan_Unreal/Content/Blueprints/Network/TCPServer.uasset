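; TCP server actor that opens a listen socket on BeginPlay and relays traffic between clients and a NetworkManager.
; Received bytes and client connections go to NetworkManager; Tick broadcasts its encoded batches to all clients when the client count is above zero.
; BeginPlay requires OnionManGameInstance but sets NetworkManager to None, and the ClientsConnectedCount increment is unwired, so this graph never raises the count.
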(event `self.ReceiveBeginPlay`
  (bind _tcpserver (`self.TCPServer`))
  (bind _listenport (`TCPServerComponent.ListenPort` _tcpserver))
  ;[1 1 1] Start
  (cast `OnionManGameInstance` (`GameplayStatics.GetGameInstance`))
  (set `self.NetworkManager` null)
  (`TCPServerComponent.StartListenServer` _tcpserver _listenport)
  (set `self.IsInitialized` true)
  (`KismetSystemLibrary.LogString` (`KismetTextLibrary.Conv_TextToString` (`|FormatText` "Open Server at IP {IP} and port {Port} " (`TCPServerComponent.ListenSocketName` _tcpserver) _listenport))))

(event `self.ReceiveTick`
  (params (DeltaSeconds :type "Float (single-precision)"))
  ;[1 1 1] Update
  (if (`self.IsInitialized`)
    (`/Engine/EditorBlueprintResources/StandardMacros.CompareInt` (`self.ClientsConnectedCount`)
      (:`>`
        (bind (_outnetworkbatches _returnvalue) (`NetworkManager.TryEncodeObjects` (`self.NetworkManager`)))
        (if _returnvalue
          (for _array_element _outnetworkbatches
            (bind _returnvalue_2 (`TCPServerComponent.Emit` (`self.TCPServer`) (`NetworkBatch.EncodedBatch` _array_element) "All"))
            (if _returnvalue_2
              (`KismetSystemLibrary.LogString` "Successfully sent a message")
              (else
                (`KismetSystemLibrary.LogString` "Failed to send a message")))))))))

(event `self.TCPServer.OnReceivedBytes`
  (params (Bytes :type "Array of Byte (by ref)"))
  ;[1 1 1] Network Events
  (`KismetSystemLibrary.LogString` "Recieved Bytes")
  (if (`self.IsInitialized`)
    (`NetworkManager.OnBytesRecieved` (`self.NetworkManager`) Bytes)))

(event `self.TCPServer.OnClientConnected`
  (params (Client :type String))
  ;[1 1 1] Network Events
  (`KismetSystemLibrary.LogString` (`KismetTextLibrary.Conv_TextToString` (`|FormatText` "NewClient conncted {client}" Client)))
  (if (`self.IsInitialized`)
    (`NetworkManager.OnClientConnected` (`self.NetworkManager`) Client)))

(fn `UserConstructionScript`)