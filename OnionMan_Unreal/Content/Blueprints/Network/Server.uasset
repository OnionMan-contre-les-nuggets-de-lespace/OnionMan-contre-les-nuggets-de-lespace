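; Server-side UDP actor that links a remote peer to the game instance's NetworkManager.
; It opens a receive socket on BeginPlay and, while disconnected, validates incoming bytes as a handshake, opens a send socket to the returned IP and replies with an acknowledgement.
; Once connected, it forwards received bytes to the NetworkManager and emits its encoded object batches every Tick.
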(event `self.ReceiveBeginPlay`
  (bind _udpcomponent (`self.UDPComponent`))
  (bind (_sendip _sendport _sendboundport _sendboundip _receiveip _receiveport) (break `UDPSettings` (`UDPComponent.Settings` _udpcomponent)))
  ;[1 1 1] Start
  (bind _asonion_man_game_instance (cast `OnionManGameInstance` (`GameplayStatics.GetGameInstance`)))
  (set `self.NetworkManager` (`OnionManGameInstance.NetworkManager` _asonion_man_game_instance))
  (bind _returnvalue (`UDPComponent.OpenReceiveSocket` _udpcomponent _receiveip _receiveport))
  (`KismetSystemLibrary.LogString` (`KismetTextLibrary.Conv_TextToString` (`|FormatText` "[UDP] Open Recieve Socket : {bool}" _returnvalue))))

(event `self.ReceiveTick`
  (params (DeltaSeconds :type "Float (single-precision)"))
  ;[1 1 1] Update
  (switch `/Game/Blueprints/Network/ConnectionState` (`self.ConnectionState`)
    (:`NewEnumerator1`
      (bind (_outnetworkbatches _returnvalue) (`NetworkManager.TryEncodeObjects` (`self.NetworkManager`)))
      (if _returnvalue
        (for _array_element _outnetworkbatches
          (bind _returnvalue_2 (`UDPComponent.EmitBytes` (`self.UDPComponent`) (`NetworkBatch.EncodedBatch` _array_element)))
          (if _returnvalue_2
            (`KismetSystemLibrary.LogString` "Successfully sent a message")
            (else
              (`KismetSystemLibrary.LogString` "Failed to send a message"))))))))

(event `self.UDPComponent.OnReceivedBytes`
  (params (Bytes :type "Array of Byte (by ref)") (IPAddress :type String) (Port :type "Integer (by ref)"))
  ;[1 1 1] Network Events
  (`KismetSystemLibrary.PrintString` (`KismetTextLibrary.Conv_TextToString` (`|FormatText` "RecievedBytes from IP {IP} and port {Port}" IPAddress Port)))
  (switch `/Game/Blueprints/Network/ConnectionState` (`self.ConnectionState`)
    (:`NewEnumerator0`
      (bind (_outencodedack _outip _returnvalue) (`NetworkManager.TryAcknoledge` (`self.NetworkManager`) Bytes))
      (if _returnvalue
        (bind _structout (setmembers `UDPSettings` :`StructRef` (`UDPComponent.Settings` (`self.UDPComponent`)) :`SendIP` _outip))
        (bind (_sendip _sendport) (break `UDPSettings` _structout))
        (bind _returnvalue_2 (`UDPComponent.OpenSendSocket` (`self.UDPComponent`) _sendip _sendport))
        (`KismetSystemLibrary.LogString` (`KismetTextLibrary.Conv_TextToString` (`|FormatText` "[UDP] Open Send Socket at IP {IP} and Port {Port} : {value}" _sendip _sendport _returnvalue_2)))
        (bind _returnvalue_3 (`UDPComponent.EmitBytes` (`self.UDPComponent`) _outencodedack))
        (if _returnvalue_3
          (set `self.IsInitialized` true)
          (set `self.ConnectionState` "NewEnumerator1")
          (`KismetSystemLibrary.LogString` "[UDP] Initialized")
          (else
            (`KismetSystemLibrary.LogString` "Failed to Emit Acknoledge")))
        (else
          (`KismetSystemLibrary.LogString` "RecievedIp was not valid"))))
    (:`NewEnumerator1`
      (`NetworkManager.OnBytesRecieved` (`self.NetworkManager`) Bytes))))

(fn `UserConstructionScript`)