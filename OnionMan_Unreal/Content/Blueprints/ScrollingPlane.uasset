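; ScrollingPlane is an actor that creates an endlessly scrolling, tinted star-texture backdrop from two planes.
; On BeginPlay it scales both planes, yaws them to the scroll direction and places the second one plane-length behind the first.
; Tick moves both, leapfrogging the leading plane behind the other once it travels that length.
; Each plane gets a random texture at start and on wrapping, through a cached dynamic material instance.
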(event `self.ReceiveBeginPlay`
  (bind _plane_0 (`self.Plane_0`))
  (bind _plane_1 (`self.Plane_1`))
  (bind _planescale (`self.PlaneScale`))
  (bind _plane_1_2 (`self.Plane_1`))
  (bind _returnvalue (`KismetMathLibrary.Normal` (`self.ScrollDirection`)))
  (bind _returnvalue_2 (`SceneComponent.K2_GetComponentLocation` (`self.Plane_0`)))
  (bind _returnvalue_3 (`KismetMathLibrary.Vector_HeadingAngle` _returnvalue))
  (bind _output_get (set `self.ScrollDirection` _returnvalue))
  (`SceneComponent.SetWorldScale3D` (`self.Plane_0`) _planescale)
  (bind _output_get_2 (set `self.BaseOffset` (* _planescale (`self.BasePlaneSize`) (* _output_get (-1.0 -1.0 -1.0)))))
  (`SceneComponent.SetWorldScale3D` _plane_1_2 (`self.PlaneScale`))
  (`SceneComponent.K2_SetWorldLocation` _plane_1_2 (+ _output_get_2 _returnvalue_2) false false)
  (set `self.BasePosition` _returnvalue_2)
  (set `self.FirstPlane` _plane_0)
  (`self.RotatePlane` _plane_0 _returnvalue_3)
  (set `self.SecondPlane` _plane_1)
  (`self.RotatePlane` _plane_1 _returnvalue_3)
  (`self.RandomizePlaneMaterial` (`self.Plane_0`))
  (`self.RandomizePlaneMaterial` (`self.Plane_1`)))

(event `self.ReceiveTick`
  (params (DeltaSeconds :type "Float (single-precision)"))
  (bind _returnvalue (* DeltaSeconds (`self.ScrollSpeed`) (`self.ScrollDirection`)))
  (`self.ScrollPlane` (`self.Plane_0`) _returnvalue)
  (`self.ScrollPlane` (`self.Plane_1`) _returnvalue)
  (if (>= (`KismetMathLibrary.VSizeXYSquared` (- (`SceneComponent.K2_GetComponentLocation` (`self.FirstPlane`)) (`self.BasePosition`))) (`KismetMathLibrary.VSizeXYSquared` (`self.BaseOffset`)))
    (`SceneComponent.K2_SetWorldLocation` (`self.FirstPlane`) (+ (`self.BaseOffset`) (`SceneComponent.K2_GetComponentLocation` (`self.SecondPlane`))) false false)
    (`self.RandomizePlaneMaterial` (`self.FirstPlane`))
    (if (== (`self.FirstPlane`) (`self.Plane_0`))
      (set `self.FirstPlane` (`self.Plane_1`))
      (set `self.SecondPlane` (`self.Plane_0`))
      (else
        (set `self.FirstPlane` (`self.Plane_0`))
        (set `self.SecondPlane` (`self.Plane_1`))))))

(fn `RandomizePlaneMaterial`
  (params (Plane :type "StaticMeshComponent Object Reference"))
  (bind _dynamicplanematerials (`self.DynamicPlaneMaterials`))
  (bind _value (`BlueprintMapLibrary.Map_Find` _dynamicplanematerials Plane))
  (if (not (`BlueprintMapLibrary.Map_Contains` _dynamicplanematerials Plane))
    (bind _returnvalue (`KismetMaterialLibrary.CreateDynamicMaterialInstance` (`PrimitiveComponent.GetMaterial` Plane 0)))
    (`BlueprintMapLibrary.Map_Add` _dynamicplanematerials Plane _returnvalue))
  (`MaterialInstanceDynamic.SetTextureParameterValue` _value "StarTexture" (`KismetArrayLibrary.Array_Random` (`self.PossibleTextures`)))
  (`MaterialInstanceDynamic.SetVectorParameterValue` _value "TexColor" (`KismetMathLibrary.Conv_ColorToLinearColor` (`self.Color`)))
  (`PrimitiveComponent.SetMaterial` Plane 0 _value))

(fn `RotatePlane`
  (params (Plane :type "StaticMeshComponent Object Reference") (Rotation :type "Float (double-precision)"))
  (bind (_returnvalue_roll _returnvalue_pitch _returnvalue_yaw) (`KismetMathLibrary.BreakRotator` (`SceneComponent.K2_GetComponentRotation` Plane)))
  (`SceneComponent.K2_SetWorldRotation` Plane (`KismetMathLibrary.MakeRotator` _returnvalue_roll _returnvalue_pitch (+ _returnvalue_yaw (`KismetMathLibrary.RadiansToDegrees` Rotation))) false false))

(fn `ScrollPlane`
  (params (PlaneToMove :type "StaticMeshComponent Object Reference") (Offset :type "Vector Structure"))
  (`SceneComponent.K2_SetWorldLocation` PlaneToMove (+ (`SceneComponent.K2_GetComponentLocation` PlaneToMove) Offset) false false))

(fn `UserConstructionScript`)